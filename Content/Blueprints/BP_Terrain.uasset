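; BP_Terrain is a sculptable terrain actor built on a procedural mesh.
; The construction script creates a welded, flat grid with collision, upward normals and a terrain material.
; The Sculpt event calls EditTerrain to offset vertices along Z within a radius of a location, weighted by a Profile curve.
; It then runs CalculateNormals, which sets each triangle's first-vertex normal from an edge cross product, and updates the mesh section.
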(event `Sculpt`
  (params (Location :type "Vector Structure"))
  (`self.EditTerrain` (- Location (`self.K2_GetActorLocation`)) (0.0 0.0 1.0) "/Game/Blueprints/Profile.Profile" 10.0)
  (`self.CalculateNormals`)
  (`ProceduralMeshComponent.UpdateMeshSection_LinearColor` :`self` (`self.ProceduralMesh`) :`Vertices` (`self.VertexFinal`) :`Normals` (`self.Normals`)))

(fn `CalculateNormals`
  (bind _vertexfinal (`self.VertexFinal`))
  (for (_array_element _array_index) (`self.Triangles`)
    (if (== (mod _array_index 3) 0)
      (bind _output (`|GetArrayItem` _vertexfinal _array_element))
      (bind _returnvalue (+ _array_index 1))
      (`KismetArrayLibrary.Array_Set` (`self.Normals`) _array_element (`KismetMathLibrary.Cross_VectorVector` (`KismetMathLibrary.Normal` (- _output (`|GetArrayItem` (`self.VertexFinal`) (`|GetArrayItem` (`self.Triangles`) (+ _returnvalue 1)))) 0.001) (`KismetMathLibrary.Normal` (- _output (`|GetArrayItem` _vertexfinal (`|GetArrayItem` (`self.Triangles`) _returnvalue))) 0.001))))))

(fn `EditTerrain`
  (params (Location :type "Vector Structure") (Direction :type "Vector Structure") (Profile :type "CurveFloat Object Reference") (Radius :type "Float (double-precision)") (Intensity :type "Float (double-precision)" :default 1.0))
  (locals (DistanceFromEditLoc :type "Float (double-precision)") (Index :type Integer))
  (bind _vertexfinal (`self.VertexFinal`))
  (for (_array_element _array_index) (`self.VertexFinal`)
    (set `local.Index` _array_index)
    (bind _output_get (set `local.DistanceFromEditLoc` (`KismetMathLibrary.Vector_Distance` _array_element (`local.Location`))))
    (if (<= _output_get (`local.Radius`))
      (`KismetArrayLibrary.Array_Set` _vertexfinal (`local.Index`) (+ (`|GetArrayItem` _vertexfinal (`local.Index`)) (* (`local.Direction`) (* (`local.Intensity`) (`CurveFloat.GetFloatValue` (`local.Profile`) (/ (`local.DistanceFromEditLoc`) (`local.Radius`)))))) true))))

(fn `UserConstructionScript`
  (`PrimitiveComponent.SetMaterial` (`self.ProceduralMesh`) 0 "/Game/Materials/M_Terrain.M_Terrain")
  (bind (_triangles _vertices _uvs) (`KismetProceduralMeshLibrary.CreateGridMeshWelded` 30 30 3.0))
  (set `self.Triangles` _triangles)
  (bind _output_get (set `self.VertexFinal` _vertices))
  (for (_ _array_index) _output_get
    (`KismetArrayLibrary.Array_Set` (`self.Normals`) _array_index (0.0 0.0 1.0) true))
  (`ProceduralMeshComponent.CreateMeshSection_LinearColor` :`self` (`self.ProceduralMesh`) :`Vertices` (`self.VertexFinal`) :`Triangles` (`self.Triangles`) :`Normals` (`self.Normals`) :`UV0` _uvs :`bCreateCollision` true))