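; BPFL_Common is a Blueprint function library with one helper, LaserRelativeRoll, which computes a motion controller laser's roll relative to a camera.
; It projects the controller-to-camera direction onto the plane perpendicular to the controller's forward vector.
; The angle from the controller's up vector comes from an arccosine in degrees, signed by the dot product with its right vector.
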(fn `LaserRelativeRoll`
  (params (Camera :type "SceneComponent Object Reference") (MotionController :type "SceneComponent Object Reference"))
  (returns (Roll :type "Float (double-precision)"))
  (bind _motioncontroller (`local.MotionController`))
  (bind _motioncontroller_2 (`local.MotionController`))
  (bind _returnvalue (`SceneComponent.GetForwardVector` _motioncontroller_2))
  (bind _returnvalue_2 (`KismetMathLibrary.Normal` (- (`SceneComponent.K2_GetComponentLocation` (`local.Camera`)) (`SceneComponent.K2_GetComponentLocation` _motioncontroller_2)) 0.001))
  (bind _returnvalue_3 (`KismetMathLibrary.Normal` (- _returnvalue_2 (* _returnvalue (`KismetMathLibrary.Dot_VectorVector` _returnvalue_2 _returnvalue))) 0.001))
  (return (* (`KismetMathLibrary.DegAcos` (`KismetMathLibrary.Dot_VectorVector` _returnvalue_3 (`SceneComponent.GetUpVector` _motioncontroller))) (`KismetMathLibrary.SignOfFloat` (`KismetMathLibrary.Dot_VectorVector` _returnvalue_3 (`SceneComponent.GetRightVector` _motioncontroller))))))