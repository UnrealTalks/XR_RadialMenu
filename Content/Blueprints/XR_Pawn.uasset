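; XR pawn that gives the player a hand-held radial menu driven by a motion controller.
; On BeginPlay it spawns BP_RadialMenu from DT_SUB_ACTORS at the controller, pitched up slightly, and attaches it.
; Right thumbstick, shoulder, trigger and Magic Leap home inputs forward navigation, selection, action and back to the menu.
; Tick repositions the menu within a narrow camera field of view for Magic Leap/HoloLens, matching controller rotation.
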(event `self.ReceiveBeginPlay`
  (bind _returnvalue (`SceneComponent.K2_GetComponentToWorld` (`self.MotionController`)))
  ;[1 1 1] Setup
  (set `MotionControllerComponent.MotionSource` "AnyHand" (`self.MotionController`))
  (bind _returnvalue_2 (`|SpawnActorFromClass` "/RadialMenu/BP_RadialMenu.BP_RadialMenu_C" (`KismetMathLibrary.MakeTransform` (.location _returnvalue) (`KismetMathLibrary.MakeRotator` (.roll (.rotation _returnvalue)) (+ (.pitch (.rotation _returnvalue)) 15.0) (.yaw (.rotation _returnvalue))) (.scale _returnvalue)) "Undefined" "OverrideRootScale" null 0.25 "/RadialMenu/DT_SUB_ACTORS.DT_SUB_ACTORS" "Example" null))
  (bind _output_get (set `self.RadialMenu` _returnvalue_2))
  (`self.K2_AttachToComponent` _output_get (`self.MotionController`) "None" "KeepRelative" "KeepRelative" "KeepRelative" true))

(event `InputAxisKey|MotionController_Right_Thumbstick_X`
  (params (AxisValue :type "Float (single-precision)"))
  (bind _radialmenu (`self.RadialMenu`))
  ;[0.1844 0.6167 1] Update Thumbstick or Touchpad
  (`/Engine/EditorBlueprintResources/StandardMacros.IsValid` _radialmenu
    (:`Is Valid`
      (`/RadialMenu/BP_RadialMenu.UpdateRadialMenu` _radialmenu AxisValue (`self.GetInputAxisKeyValue`)))))

(event `Key|MotionController_Right_Shoulder`
  (params (Key :type "Key Structure"))
  (bind _radialmenu (`self.RadialMenu`))
  ;[1 0.8843 0.4247] Select
  (:`Pressed`
    (`/Engine/EditorBlueprintResources/StandardMacros.IsValid` _radialmenu
      (:`Is Valid`
        (`/RadialMenu/BP_RadialMenu.ShoulderSelect` _radialmenu)))))

(event `Key|MotionController_Right_Trigger`
  (params (Key :type "Key Structure"))
  (bind _radialmenu (`self.RadialMenu`))
  ;[0 1 0.03953] Action
  (:`Pressed`
    (`/Engine/EditorBlueprintResources/StandardMacros.IsValid` _radialmenu
      (:`Is Valid`
        (`/RadialMenu/BP_RadialMenu.TriggerAction` _radialmenu (`SceneComponent.K2_GetComponentToWorld` (`self.MotionController`))))))
  (:`Released`
    (`/Engine/EditorBlueprintResources/StandardMacros.IsValid` _radialmenu
      (:`Is Valid`
        (`/RadialMenu/BP_RadialMenu.TriggerActionRelease` _radialmenu)))))

(event `Key|MagicLeap_Right_HomeButton`
  (params (Key :type "Key Structure"))
  (bind _radialmenu (`self.RadialMenu`))
  ;[1 0.03922 0] Go back one level
  (:`Pressed`
    (`/Engine/EditorBlueprintResources/StandardMacros.IsValid` _radialmenu
      (:`Is Valid`
        (`/RadialMenu/BP_RadialMenu.GoBack` _radialmenu)))))

(event `self.ReceiveTick`
  (params (DeltaSeconds :type "Float (single-precision)"))
  (bind _motioncontroller (`self.MotionController`))
  (bind _rootcomponent (`Actor.RootComponent` (`self.RadialMenu`)))
  ;[0.276 0.276 0.276] Optional: keep radial menu in view for Magic Leap / Hololens
  (bind _worldlocation (`/RadialMenu/BPFL_RadialMenuMath.FindLocationToKeepMenuInView` 0.0 _motioncontroller (16.0 11.0) (`self.Camera`)))
  (`SceneComponent.K2_SetWorldLocation` _rootcomponent _worldlocation false false)
  (`SceneComponent.K2_SetWorldLocationAndRotation` _rootcomponent _worldlocation (`SceneComponent.K2_GetComponentRotation` _motioncontroller) false false))

(fn `UserConstructionScript`)